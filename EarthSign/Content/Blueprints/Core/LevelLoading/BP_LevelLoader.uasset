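; BP_LevelLoader is a Blueprint that switches between streaming levels, keeping track of one loaded level at a time by name.
; On BeginPlay it force-loads the level stored in CurrentLevelLoaded.
; LoadLevel skips repeat requests unless forced, flags the previous level to unload and hide, then flags the new one to load and show.
; An invalid name other than "None" prints an error.
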(event EventBeginPlay
  (CallFunction|LoadLevel (Variables|Default|GetCurrent%20Level%20Loaded) true))

(fn ConstructionScript)

(fn LoadLevel
  (params (Level :type String) (Force%20Load :type Boolean))
  (if (or (Utilities|Enum|NotEqual(Enum) Level (Variables|Default|GetCurrent%20Level%20Loaded)) Force%20Load)
    (Utilities|FlowControl|Sequence
      (:then_0
        (Utilities|IsValid (Class|GameplayStatics|GetStreamingLevel (Utilities|String|StringToName (Variables|Default|GetCurrent%20Level%20Loaded)))
          (:Is%20Valid
            (Variables|/Script/Engine.LevelStreaming|SetbShouldBeLoaded (Class|GameplayStatics|GetStreamingLevel (Utilities|String|StringToName (Variables|Default|GetCurrent%20Level%20Loaded))) false)
            (Variables|/Script/Engine.LevelStreaming|SetbShouldBeVisible (Class|GameplayStatics|GetStreamingLevel (Utilities|String|StringToName (Variables|Default|GetCurrent%20Level%20Loaded))) false))))
      (:then_1
        (bind _output_get (Variables|Default|SetCurrent%20Level%20Loaded Level))
        (Utilities|IsValid (Class|GameplayStatics|GetStreamingLevel (Utilities|String|StringToName _output_get))
          (:Is%20Valid
            (Variables|/Script/Engine.LevelStreaming|SetbShouldBeLoaded (Class|GameplayStatics|GetStreamingLevel (Utilities|String|StringToName _output_get)) true)
            (Variables|/Script/Engine.LevelStreaming|SetbShouldBeVisible (Class|GameplayStatics|GetStreamingLevel (Utilities|String|StringToName _output_get)) true))
          (:Is%20Not%20Valid
            (if (not (Utilities|Enum|Equal(Enum) (Variables|Default|GetCurrent%20Level%20Loaded) "None"))
              (Development|PrintString (Utilities|String|Append "Error: BP_LevelLoader>LoadLevel() - Invalid Level name " Level)))))))))