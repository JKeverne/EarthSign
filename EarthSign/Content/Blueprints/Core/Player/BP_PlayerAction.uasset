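; BP_PlayerAction is the player input actor that runs selected grid actions on the tile under the cursor.
; After a short startup delay, Tick updates the hovered BP_Grid tile, moving a tile state to it and firing a change event.
; Left and right clicks execute their action actors on the hovered tile, repeating as the cursor drags across tiles.
; SetSelectedActions destroys and respawns both action actors, then broadcasts the change.
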(event Custom|OnHoveredTileChange
  ;[0.25 0 0] Redo with Enhanced Input Actions
  (Utilities|FlowControl|Sequence
    (:then_0
      (if (Variables|Default|GetIsLeftClickDown)
        (Utilities|IsValid (Variables|Default|GetSelectedAction_LMB)
          (:Is%20Valid
            (Default|ExecuteAction (Variables|Default|GetSelectedAction_LMB) (Variables|Default|GetHovered%20Tile))))))
    (:then_1
      (if (Variables|Default|GetIsRightClickDown)
        (Utilities|IsValid (Variables|Default|GetSelectedAction_RMB)
          (:Is%20Valid
            (Default|ExecuteAction (Variables|Default|GetSelectedAction_RMB) (Variables|Default|GetHovered%20Tile))))))))

(event EventBeginPlay
  (bind _returnvalue (Actor|GetActorOfClass "/Game/Blueprints/Core/Grid/BP_Grid.BP_Grid_C"))
  (Variables|Default|SetGrid _returnvalue)
  (Input|EnableInput (Game|GetPlayerController 0))
  (Utilities|FlowControl|Delay 0.2)
  (Utilities|FlowControl|Gate true) ; enters at Open
)

(event EventTick
  (params (DeltaSeconds :type Float%20%28single-precision%29))
  (Utilities|FlowControl|Gate true
    (:Exit
      (CallFunction|UpdateTileUnderCursor))))

(event Input|MouseEvents|LeftMouseButton
  (params (Key :type Key%20Structure :default "None"))
  ;[0.25 0 0] Redo with Enhanced Input Actions
  (:Pressed
    (Variables|Default|SetIsLeftClickDown true)
    (CallFunction|UpdateTileUnderCursor)
    (Utilities|IsValid (Variables|Default|GetSelectedAction_LMB)
      (:Is%20Valid
        (Default|ExecuteAction (Variables|Default|GetSelectedAction_LMB) (Variables|Default|GetHovered%20Tile)))))
  (:Released
    (Variables|Default|SetIsLeftClickDown false)))

(event Input|MouseEvents|RightMouseButton
  (params (Key :type Key%20Structure :default "None"))
  ;[0.25 0 0] Redo with Enhanced Input Actions
  (:Pressed
    (Variables|Default|SetIsRightClickDown true)
    (CallFunction|UpdateTileUnderCursor)
    (Utilities|IsValid (Variables|Default|GetSelectedAction_RMB)
      (:Is%20Valid
        (Default|ExecuteAction (Variables|Default|GetSelectedAction_RMB) (Variables|Default|GetHovered%20Tile)))))
  (:Released
    (Variables|Default|SetIsRightClickDown false)))

(fn ConstructionScript)

(fn UpdateTileUnderCursor
  (bind _grid (Variables|Default|GetGrid))
  (bind _index (Default|GetTileIndexUnderCursor _grid))
  (if (!= _index (Variables|Default|GetHovered%20Tile))
    (Default|RemoveStatefromTile _grid (Variables|Default|GetHovered%20Tile) "NewEnumerator1")
    (bind _output_get (Variables|Default|SetHovered%20Tile _index))
    (Default|AddStatetoTile _grid _output_get "NewEnumerator1")
    (CallFunction|OnHoveredTileChange)))

(fn SetSelectedActions
  (params (Left%20Mouse%20Button :type BP%20Action%20Class%20Reference) (Right%20Mouse%20Button :type BP%20Action%20Class%20Reference))
  (Utilities|FlowControl|Sequence
    (:then_0
      (Utilities|IsValid (Variables|Default|GetSelectedAction_LMB)
        (:Is%20Valid
          (Actor|DestroyActor (Variables|Default|GetSelectedAction_LMB))
          (Variables|Default|SetSelectedAction_LMB 0))
        (:Is%20Not%20Valid
          _))
      (if (Utilities|IsValidClass Left%20Mouse%20Button)
        (bind _returnvalue (Game|SpawnActorfromClass Left%20Mouse%20Button (Math|Transform|MakeTransform "0, 0, 0" "0, 0, 0" "1.000000,1.000000,1.000000") "AlwaysSpawn" "MultiplyWithRoot" 0 self 0))
        (Variables|Default|SetSelectedAction_LMB _returnvalue)))
    (:then_1
      (Utilities|IsValid (Variables|Default|GetSelectedAction_RMB)
        (:Is%20Valid
          (Actor|DestroyActor (Variables|Default|GetSelectedAction_RMB))
          (Variables|Default|SetSelectedAction_RMB 0))
        (:Is%20Not%20Valid
          _))
      (if (Utilities|IsValidClass Right%20Mouse%20Button)
        (bind _returnvalue_2 (Game|SpawnActorfromClass Right%20Mouse%20Button (Math|Transform|MakeTransform "0, 0, 0" "0, 0, 0" "1.000000,1.000000,1.000000") "AlwaysSpawn" "MultiplyWithRoot" 0 self 0))
        (Variables|Default|SetSelectedAction_RMB _returnvalue_2)))
    (:then_2
      (Default|CallOnSelectedActionsChanged (Variables|Default|GetSelectedAction_LMB) (Variables|Default|GetSelectedAction_RMB)))))