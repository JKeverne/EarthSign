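; Player grid action that adds a new tile to the grid at a given index.
; ExecuteAction runs only when the grid reports that index as not valid, so existing tiles are left untouched.
; It traces for ground at the index's location, then adds a tile of a fixed type at the traced location, taking rotation and scale from the grid.
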(fn ConstructionScript
  (|CallParentFunction))

(fn ExecuteAction
  (params (Index :type Int%20Point%20Structure))
  (bind _player_actions (Variables|Default|GetPlayer%20Actions))
  (bind _grid (Variables|/Game/Blueprints/Core/Player/BP_PlayerAction.BP_PlayerAction_C|GetGrid _player_actions))
  (if (not (Default|IsIndexValid (Variables|/Game/Blueprints/Core/Player/BP_PlayerAction.BP_PlayerAction_C|GetGrid (Variables|Default|GetPlayer%20Actions)) Index))
    (bind _out_location (Default|TraceforGround _grid (Default|GetTileLocationfromGridIndex _grid Index)))
    (Default|AddGridTile (Variables|/Game/Blueprints/Core/Player/BP_PlayerAction.BP_PlayerAction_C|GetGrid (Variables|Default|GetPlayer%20Actions)) (Utilities|Struct|MakeS_TileData Index "NewEnumerator1" (Math|Transform|MakeTransform _out_location (Default|GetTileRotationfromGridIndex _grid Index) (Default|GetTileScale _grid)) "NewEnumerator0"))))