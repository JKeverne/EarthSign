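; Player action that changes the type of a grid tile at a given index.
; When executed, it checks that the index is valid and looks up the existing tile data in the grid.
; It then re-adds the tile with the action's TileType, keeping its index, transform and states.
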(fn ConstructionScript
  (|CallParentFunction))

(fn ExecuteAction
  (params (Index :type Int%20Point%20Structure))
  (if (Default|IsIndexValid (Variables|/Game/Blueprints/Core/Player/BP_PlayerAction.BP_PlayerAction_C|GetGrid (Variables|Default|GetPlayer%20Actions)) Index)
    (LocalVariables|SetData (.Value (Utilities|Map|Find (Variables|/Game/Blueprints/Core/Grid/BP_Grid.BP_Grid_C|GetGrid%20Tiles (Variables|/Game/Blueprints/Core/Player/BP_PlayerAction.BP_PlayerAction_C|GetGrid (Variables|Default|GetPlayer%20Actions))) Index)))
    (Default|AddGridTile (Variables|/Game/Blueprints/Core/Player/BP_PlayerAction.BP_PlayerAction_C|GetGrid (Variables|Default|GetPlayer%20Actions)) (Utilities|Struct|MakeS_TileData (.index (LocalVariables|GetData)) (Variables|Default|GetTile%20Type) (.transform (LocalVariables|GetData)) (.states (LocalVariables|GetData))))))