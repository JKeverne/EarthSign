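; Player grid action that selects a tile, holding a single selected tile index on PlayerActions.
; Executing it on a new index moves the grid's selection state from the previous tile to that one, while executing on the already selected tile clears it.
; On destruction it executes with the sentinel index (-999, -999), which removes the current selection's state.
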(event EventDestroyed
  (CallFunction|ExecuteAction (Utilities|Struct|MakeIntPoint -999 -999)))

(fn ConstructionScript
  (|CallParentFunction))

(fn ExecuteAction
  (params (Index :type Int%20Point%20Structure))
  (bind _player_actions (Variables|Default|GetPlayer%20Actions))
  (bind _player_actions_2 (Variables|Default|GetPlayer%20Actions))
  (bind _player_actions_3 (Variables|Default|GetPlayer%20Actions))
  (if (!= (Variables|/Game/Blueprints/Core/Player/BP_PlayerAction.BP_PlayerAction_C|GetSelected%20Tile (Variables|Default|GetPlayer%20Actions)) Index)
    (Default|RemoveStatefromTile (Variables|/Game/Blueprints/Core/Player/BP_PlayerAction.BP_PlayerAction_C|GetGrid _player_actions) (Variables|/Game/Blueprints/Core/Player/BP_PlayerAction.BP_PlayerAction_C|GetSelected%20Tile _player_actions) "NewEnumerator2")
    (Variables|/Game/Blueprints/Core/Player/BP_PlayerAction.BP_PlayerAction_C|SetSelected%20Tile (Variables|Default|GetPlayer%20Actions) Index)
    (Default|AddStatetoTile (Variables|/Game/Blueprints/Core/Player/BP_PlayerAction.BP_PlayerAction_C|GetGrid _player_actions_3) (Variables|/Game/Blueprints/Core/Player/BP_PlayerAction.BP_PlayerAction_C|GetSelected%20Tile _player_actions_3) "NewEnumerator2")
    (else
      (Default|RemoveStatefromTile (Variables|/Game/Blueprints/Core/Player/BP_PlayerAction.BP_PlayerAction_C|GetGrid _player_actions_2) (Variables|/Game/Blueprints/Core/Player/BP_PlayerAction.BP_PlayerAction_C|GetSelected%20Tile _player_actions_2) "NewEnumerator2")
      (Variables|/Game/Blueprints/Core/Player/BP_PlayerAction.BP_PlayerAction_C|SetSelected%20Tile (Variables|Default|GetPlayer%20Actions) (Utilities|Struct|MakeIntPoint -999 -999)))))