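; A player camera pawn with zoom, planar movement and yaw rotation controls.
; On BeginPlay it adds the camera Enhanced Input mapping context and seeds desired location, rotation and spring arm length from current values.
; Input actions only adjust those targets: clamped zoom, translation along the actor's forward and right vectors, and stepped rotation on press.
; Tick smoothly interpolates the spring arm and actor transform toward the targets.
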(event Input|EnhancedActionEvents|EnhancedInputActionIA_Camera_Zoom
  (params (ActionValue :type Float%20%28double-precision%29) (ElapsedSeconds :type Float%20%28double-precision%29) (TriggeredSeconds :type Float%20%28double-precision%29) (InputAction :type Input%20Action%20Object%20Reference :default "/Game/Input/InputActions/IA_Camera_Zoom.IA_Camera_Zoom"))
  ;[0 0 0.15 0.5] Camera
  ;;[0.15 0.15 0.15 0.5] Camera Zoom
  (Variables|Camera|SetZoomDesired (Math|Float|Clamp(Float) (+ (Variables|Camera|GetZoomDesired) (* ActionValue (Variables|Camera|GetZoomSpeed))) (Variables|Camera|GetZoomMin) (Variables|Camera|GetZoomMax))))

(event Input|EnhancedActionEvents|EnhancedInputActionIA_Camera_RotateLeft
  (params (ActionValue :type Boolean) (ElapsedSeconds :type Float%20%28double-precision%29) (TriggeredSeconds :type Float%20%28double-precision%29) (InputAction :type Input%20Action%20Object%20Reference :default "/Game/Input/InputActions/IA_Camera_RotateLeft.IA_Camera_RotateLeft"))
  ;[0 0 0.15 0.5] Camera
  ;;[0.15 0.15 0.15 0.5] Camera Rotation
  (:Started
    (Variables|Camera|SetRotationDesired (Math|Rotator|CombineRotators (Variables|Camera|GetRotationDesired) (Math|Rotator|MakeRotator 0.0 0.0 (Variables|Camera|GetRotationSpeed))))))

(event Input|EnhancedActionEvents|EnhancedInputActionIA_Camera_BackwardForward
  (params (ActionValue :type Float%20%28double-precision%29) (ElapsedSeconds :type Float%20%28double-precision%29) (TriggeredSeconds :type Float%20%28double-precision%29) (InputAction :type Input%20Action%20Object%20Reference :default "/Game/Input/InputActions/IA_Camera_BackwardForward.IA_Camera_BackwardForward"))
  ;[0 0 0.15 0.5] Camera
  ;;[0.15 0.15 0.15 0.5] Camera Translation
  (Variables|Camera|SetLocationDesired (+ (Variables|Camera|GetLocationDesired) (* (* ActionValue (Variables|Camera|GetTranslationSpeed)) (Transformation|GetActorForwardVector)))))

(event Input|EnhancedActionEvents|EnhancedInputActionIA_Camera_LeftRight
  (params (ActionValue :type Float%20%28double-precision%29) (ElapsedSeconds :type Float%20%28double-precision%29) (TriggeredSeconds :type Float%20%28double-precision%29) (InputAction :type Input%20Action%20Object%20Reference :default "/Game/Input/InputActions/IA_Camera_LeftRight.IA_Camera_LeftRight"))
  ;[0 0 0.15 0.5] Camera
  ;;[0.15 0.15 0.15 0.5] Camera Translation
  (Variables|Camera|SetLocationDesired (+ (Variables|Camera|GetLocationDesired) (* (* ActionValue (Variables|Camera|GetTranslationSpeed)) (Transformation|GetActorRightVector)))))

(event Input|EnhancedActionEvents|EnhancedInputActionIA_Camera_RotateRight
  (params (ActionValue :type Boolean) (ElapsedSeconds :type Float%20%28double-precision%29) (TriggeredSeconds :type Float%20%28double-precision%29) (InputAction :type Input%20Action%20Object%20Reference :default "/Game/Input/InputActions/IA_Camera_RotateRight.IA_Camera_RotateRight"))
  ;[0 0 0.15 0.5] Camera
  ;;[0.15 0.15 0.15 0.5] Camera Rotation
  (:Started
    (Variables|Camera|SetRotationDesired (Math|Rotator|CombineRotators (Variables|Camera|GetRotationDesired) (Math|Rotator|MakeRotator 0.0 0.0 (* (Variables|Camera|GetRotationSpeed) -1.0))))))

(event EventBeginPlay
  ;[0 0.5 0 0.5] Begin Play
  (bind _asbp_player_controller (Utilities|Casting|CastToBP_PlayerController (Pawn|GetController)))
  (Utilities|IsValid _asbp_player_controller
    (:Is%20Valid
      (Input|AddMappingContext (PlayerController|LocalPlayerSubsystems|GetEnhancedInputLocalPlayerSubsystem _asbp_player_controller) "/Game/Input/IMC_CameraControls.IMC_CameraControls" 0 "(bIgnoreAllPressedKeysUntilRelease=True,bForceImmediately=False,bNotifyUserSettings=False)")
      ;;[0.15 0.15 0.15 0.5] Set Default Camera Values
      (Variables|Camera|SetLocationDesired (Transformation|GetActorLocation))
      (Variables|Camera|SetZoomDesired (Variables|/Script/Engine.SpringArmComponent|GetTargetArmLength (Variables|Default|GetSpringArm)))
      (Variables|Camera|SetRotationDesired (Transformation|GetActorRotation)))))

(event EventTick
  (params (DeltaSeconds :type Float%20%28single-precision%29))
  (bind _springarm (Variables|Default|GetSpringArm))
  ;[0.15 0.15 0.15 0.5] Tick
  (Variables|/Script/Engine.SpringArmComponent|SetTargetArmLength _springarm (Math|Interpolation|FInterpTo (Variables|/Script/Engine.SpringArmComponent|GetTargetArmLength _springarm) (Variables|Camera|GetZoomDesired) DeltaSeconds (Variables|Camera|GetZoomInterpSpeed)))
  (Transformation|SetActorLocation (Math|Interpolation|VInterpTo (Transformation|GetActorLocation) (Variables|Camera|GetLocationDesired) DeltaSeconds (Variables|Camera|GetTranslationInterpSpeed)) false false)
  (Transformation|SetActorRotation (Math|Interpolation|RInterpTo (Transformation|GetActorRotation) (Variables|Camera|GetRotationDesired) DeltaSeconds (Variables|Camera|GetRotationInterpSpeed))))

(fn ConstructionScript)