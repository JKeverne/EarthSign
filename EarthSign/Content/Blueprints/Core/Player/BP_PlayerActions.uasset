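; Player action actor that handles tile hovering and mouse-click tile marking on the BP_Grid found in the level.
; After a short startup delay, a gate lets Tick query the tile under the cursor, moving the hover state only when that tile changes.
; Left and right clicks add or remove a second state on the hovered tile, using legacy key events noted for replacement with Enhanced Input.
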(event EventBeginPlay
  (bind _returnvalue (Actor|GetActorOfClass "/Game/Blueprints/Core/Grid/BP_Grid.BP_Grid_C"))
  (Variables|Default|SetGrid _returnvalue)
  (Input|EnableInput (Game|GetPlayerController 0))
  (Utilities|FlowControl|Delay 0.2)
  (Utilities|FlowControl|Gate true) ; enters at Open
)

(event EventTick
  (params (DeltaSeconds :type Float%20%28single-precision%29))
  (Utilities|FlowControl|Gate true
    (:Exit
      (CallFunction|UpdateTileUnderCursor))))

(event Input|MouseEvents|LeftMouseButton
  (params (Key :type Key%20Structure :default "None"))
  ;[0.25 0 0] Redo with Enhanced Input Actions
  (:Pressed
    (Default|AddStatetoTile (Variables|Default|GetGrid) (Variables|Default|GetHovered%20Tile) "NewEnumerator2")))

(event Input|MouseEvents|RightMouseButton
  (params (Key :type Key%20Structure :default "None"))
  ;[0.25 0 0] Redo with Enhanced Input Actions
  (:Pressed
    (Default|RemoveStatefromTile (Variables|Default|GetGrid) (Variables|Default|GetHovered%20Tile) "NewEnumerator2")))

(fn ConstructionScript)

(fn UpdateTileUnderCursor
  (bind _grid (Variables|Default|GetGrid))
  (bind _index (Default|GetTileIndexUnderCursor _grid))
  (if (!= _index (Variables|Default|GetHovered%20Tile))
    (Default|RemoveStatefromTile _grid (Variables|Default|GetHovered%20Tile) "NewEnumerator1")
    (bind _output_get (Variables|Default|SetHovered%20Tile _index))
    (Default|AddStatetoTile _grid _output_get "NewEnumerator1")))